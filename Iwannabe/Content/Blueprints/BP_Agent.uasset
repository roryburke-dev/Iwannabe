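; BP_Agent is an AI agent that uses AIMoveTo to travel to a stored target position.
; BeginPlay sets the target to the agent's own nav location, and Tick reissues the move every frame while IsAtTarget is false.
; On success it prints a debug message, switches the target to a hardcoded point and immediately clears the flag, so the move requests continue.
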(event `self.ReceiveBeginPlay`
  (set `self.TargetPosition` (`self.GetNavAgentLocation`))
  (set `self.IsAtTarget` false))

(event `self.ReceiveTick`
  (params (DeltaSeconds :type "Float (single-precision)"))
  (if (not (`self.IsAtTarget`))
    (`|AIMoveTo` self (`self.TargetPosition`) null
      (:`OnSuccess`
        (set `self.IsAtTarget` true)
        (if true
          (`KismetSystemLibrary.PrintString` "Agent is at their target")
          (set `self.TargetPosition` (-2000.0 2000.0 0.0))
          (set `self.IsAtTarget` false))))))

(fn `UserConstructionScript`)